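; TronCube is an actor that eases vertically to a fixed world height, keeping its X and Y position.
; Each Tick, while IsRaised is false, it interpolates its current Z toward the target with FInterpTo and moves itself without sweeping.
; Once the interpolated value equals the target, it sets IsRaised to stop further movement; the construction script is empty.
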(event `self.ReceiveTick`
  (params (DeltaSeconds :type "Float (single-precision)"))
  (bind _returnvalue (`KismetMathLibrary.FInterpTo` (.z (`self.K2_GetActorLocation`)) 50.0 (`GameplayStatics.GetWorldDeltaSeconds`) 2.0))
  (if (not (`self.IsRaised?`))
    (`self.K2_SetActorLocation` (`KismetMathLibrary.MakeVector` (.x (`self.K2_GetActorLocation`)) (.y (`self.K2_GetActorLocation`)) _returnvalue))
    (if (== _returnvalue 50.0)
      (set `self.IsRaised?` true))))

(fn `UserConstructionScript`)